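; Gameplay ability that casts an energy bolt projectile toward the location under the mouse cursor.
; A custom target-data task supplies the hit location, and the avatar turns to face it through the F1 combat interface.
; The cast montage plays while a gameplay event wait spawns the projectile when the montage's EnergyBolt event arrives.
; The ability ends when the montage completes, blends out, is interrupted or is cancelled.
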(event `self.K2_ActivateAbility`
  (bind (_asynctaskproxy _datahandle) (`F1TargetDataUnderMouse.CreateTargetDataUnderMouse`)
    (:`ValidData`
      (set `self.ProjectileTargetLocation` (`.Location` (`GameplayStatics.BreakHitResult` (`AbilitySystemBlueprintLibrary.GetHitResultFromTargetData` _datahandle))))
      (bind _asf1combat_interface (cast `F1CombatInterface` (`self.GetAvatarActorFromActorInfo`)))
      (`F1CombatInterface.UpdateFacingTarget` _asf1combat_interface (`self.ProjectileTargetLocation`))
      (`AbilityTask_PlayMontageAndWait.CreatePlayMontageAndWaitProxy` "None" "/Game/Blueprints/Character/Hero/Dekker/AM_CastEnergyBolt.AM_CastEnergyBolt"
        (:`then`
          (`AbilityTask_WaitGameplayEvent.WaitGameplayEvent` (struct :`TagName` "Event.Montage.EnergyBolt") null
            (:`EventReceived`
              (`self.SpawnProjectile` (`self.ProjectileTargetLocation`)))))
        (:`OnCompleted`
          (`self.K2_EndAbility` :!label _label))
        (:`OnBlendOut`
          (goto _label))
        (:`OnInterrupted`
          (goto _label))
        (:`OnCancelled`
          (goto _label))))))