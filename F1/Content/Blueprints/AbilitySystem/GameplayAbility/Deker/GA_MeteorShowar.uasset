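; Gameplay ability for Deker that casts a meteor shower at the location under the mouse.
; It flattens the hit point to a fixed height, then moves the avatar until it is within casting range.
; On arrival it commits, turns to face the target and plays the cast montage, whose gameplay event triggers the area actor spawn.
; The ability ends when the montage finishes or breaks off, or when commit fails.
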(event `self.K2_ActivateAbility`
  (bind (_asynctaskproxy _datahandle) (`F1TargetDataUnderMouse.CreateTargetDataUnderMouse`)
    (:`ValidData`
      (set `self.TargetLocation` (`KismetMathLibrary.MakeVector` (.x (`.Location` (`GameplayStatics.BreakHitResult` (`AbilitySystemBlueprintLibrary.GetHitResultFromTargetData` _datahandle)))) (.y (`.Location` (`GameplayStatics.BreakHitResult` (`AbilitySystemBlueprintLibrary.GetHitResultFromTargetData` _datahandle)))) 20.0))
      (bind _asf1combat_interface (cast `F1CombatInterface` (`self.GetAvatarActorFromActorInfo`)))
      (`F1MoveToTarget.MoveToTarget` null (`self.TargetLocation`) 800.0
        (:`OnReached`
          (bind _returnvalue (`self.K2_CommitAbility`))
          (if _returnvalue
            (`F1CombatInterface.UpdateFacingTarget` _asf1combat_interface (`self.TargetLocation`))
            (`AbilityTask_PlayMontageAndWait.CreatePlayMontageAndWaitProxy` "None" "/Game/Blueprints/Character/Hero/Dekker/AM_CastMeteorShowar.AM_CastMeteorShowar"
              (:`then`
                (`AbilityTask_WaitGameplayEvent.WaitGameplayEvent` (struct :`TagName` "Event.Montage.MeteorShowar") null
                  (:`EventReceived`
                    (`self.SpawnAreaActor` (`self.TargetLocation`)))))
              (:`OnCompleted`
                (`self.K2_EndAbility` :!label _label))
              (:`OnBlendOut`
                (goto _label))
              (:`OnInterrupted`
                (goto _label))
              (:`OnCancelled`
                (goto _label)))
            (else
              (`self.K2_EndAbility`))))))))